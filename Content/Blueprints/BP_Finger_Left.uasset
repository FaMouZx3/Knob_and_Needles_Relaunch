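; Left pinball flipper that swings up automatically when a Pinball actor overlaps its Box, then swings back down two seconds later.
; BeginPlay stores the root's world rotation and sets the timeline play rate from AnimPlayRate.
; LeftFingerUp plays a timeline that lerps yaw from that rotation by RotationVariance, and LeftFingerDown reverses it.
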(event `self.ReceiveBeginPlay`
  (set `self.InitialRot` (`SceneComponent.K2_GetComponentRotation` (`self.DefaultSceneRoot`)))
  (`TimelineComponent.SetPlayRate` (`self.Timeline_0`) (`self.AnimPlayRate`)))

(event `Left Finger Up`
  (bind _initialrot (`self.InitialRot`))
  (bind (_direction _rotation) (`Timeline|Timeline_0` :!via `PlayFromStart` :!label _label)
    (:`Update`
      (`SceneComponent.K2_SetWorldRotation` (`self.DefaultSceneRoot`) (`KismetMathLibrary.RLerp` _initialrot (`KismetMathLibrary.MakeRotator` (.roll _initialrot) (.pitch _initialrot) (+ (.yaw _initialrot) (`self.RotationVariance`))) _rotation) false false))))

(event `Left Finger Down`
  (goto _label :!via `Reverse`))

(event `self.Box.OnComponentBeginOverlap`
  (params (OverlappedComponent :type "PrimitiveComponent Object Reference") (OtherActor :type "Actor Object Reference") (OtherComp :type "PrimitiveComponent Object Reference") (OtherBodyIndex :type Integer) (bFromSweep :type Boolean) (SweepResult :type "HitResult Structure (by ref)"))
  (cast `/Game/Blueprints/Pinball` OtherActor)
  (if true
    (`self.Left Finger Up`)
    (`KismetSystemLibrary.Delay` 2.0)
    (`self.Left Finger Down`)))

(fn `UserConstructionScript`)