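; BP_Cannon is a cannon actor that swivels and fires physics pinballs.
; On BeginPlay, a timeline sweeps its yaw between limits set relative to the starting rotation.
; The FireCannon event waits a short random delay, spawns a BP_Pinball at the Scene component, then applies an impulse along the mesh's forward vector, scaled by CanonForce.
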(event `self.ReceiveBeginPlay`
  (bind (_returnvalue_roll _returnvalue_pitch _returnvalue_yaw) (`KismetMathLibrary.BreakRotator` (`self.K2_GetActorRotation`)))
  (bind _yaw (`self.Yaw`))
  (set `self.Yaw` _returnvalue_yaw)
  (bind (_direction _can_rot) (`Timeline|Cannon_rotation`)
    (:`Update`
      (`self.K2_SetActorRotation` (`KismetMathLibrary.MakeRotator` 0.0 0.0 (`KismetMathLibrary.Lerp` (- _yaw (`self.Rot_min`)) (+ _yaw (`self.Rot_Max`)) _can_rot))))))

(event `FireCannon`
  (`KismetSystemLibrary.Delay` (`KismetMathLibrary.RandomFloatInRange` 0.5 1.5))
  (bind _returnvalue (`|SpawnActorFromClass` "/Game/Blueprints/Events/BP_Pinball.BP_Pinball_C" (`SceneComponent.K2_GetComponentToWorld` (`self.Scene`)) "Undefined" "OverrideRootScale" null null))
  (`PrimitiveComponent.AddImpulse` (`/Game/Blueprints/Events/BP_Pinball.Sphere` _returnvalue) (* (`SceneComponent.GetForwardVector` (`self.StaticMesh`)) (`self.CanonForce`)) "None" false))

(fn `UserConstructionScript`)