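; BP_Bumper_Left is a bumper that knocks away the pinball or ninja character that overlaps its Box component.
; A BP_Pinball gets an impulse on its cannonball mesh along the box's forward vector, scaled by Strength.
; A BP_CH_Ninja is launched along the same vector and takes Damage through GotHit.
; Both hits play a quiet 2D rubber impact sound.
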(event `self.Box.OnComponentBeginOverlap`
  (params (OverlappedComponent :type "PrimitiveComponent Object Reference") (OtherActor :type "Actor Object Reference") (OtherComp :type "PrimitiveComponent Object Reference") (OtherBodyIndex :type Integer) (bFromSweep :type Boolean) (SweepResult :type "HitResult Structure (by ref)"))
  (bind _returnvalue (`SceneComponent.GetForwardVector` (`self.Box`)))
  (bind _asbp_pinball (cast `/Game/Blueprints/Events/BP_Pinball` OtherActor)
    (:`then`
      (`PrimitiveComponent.AddImpulse` (`/Game/Blueprints/Events/BP_Pinball.SM_CannonBall` _asbp_pinball) (* _returnvalue (* (`self.Strength`) 100000.0)) "None" false))
    (:`CastFailed`
      (bind _asbp_ch_ninja (cast `/Game/Blueprints/Characters/BP_CH_Ninja` OtherActor))
      (`Character.LaunchCharacter` _asbp_ch_ninja (* _returnvalue (* (`self.Strength`) 250.0)) false false)
      (`/Game/Blueprints/Characters/BP_CH_Ninja.GotHit` _asbp_ch_ninja (`self.Damage`))))
  (`GameplayStatics.PlaySound2D` "/Game/Audio/Effects/Rubber_Hit__1.Rubber_Hit__1" 0.2))

(fn `UserConstructionScript`)