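; Trigger volume that randomly flips the pinball fingers when a pinball enters its box.
; On BeginPlay it caches the first left and right finger actors found in the level.
; On overlap, nested weighted coin flips choose no action, both fingers, left only or right only, with chosen fingers raised briefly then lowered.
; The construction script sizes the box from TriggerExtent.
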(event `self.ReceiveBeginPlay`
  (bind _outactors (`GameplayStatics.GetAllActorsOfClass` "/Game/Blueprints/Events/BP_Finger_Left.BP_Finger_Left_C"))
  (set `self.LeftFinger` (`|GetArrayItem` _outactors))
  (bind _outactors_2 (`GameplayStatics.GetAllActorsOfClass` "/Game/Blueprints/Events/BP_Finger_Right.BP_Finger_Right_C"))
  (set `self.RightFinger` (`|GetArrayItem` _outactors_2)))

(event `self.Box.OnComponentBeginOverlap`
  (params (OverlappedComponent :type "PrimitiveComponent Object Reference") (OtherActor :type "Actor Object Reference") (OtherComp :type "PrimitiveComponent Object Reference") (OtherBodyIndex :type Integer) (bFromSweep :type Boolean) (SweepResult :type "HitResult Structure (by ref)"))
  (cast `/Game/Blueprints/Events/BP_Pinball` OtherActor)
  (if (`KismetMathLibrary.RandomBoolWithWeight` 0.5)
    _
    (elif (`KismetMathLibrary.RandomBoolWithWeight` 0.5)
      (`/Game/Blueprints/Events/BP_Finger_Left.Left Finger Up` (`self.LeftFinger`))
      (`/Game/Blueprints/Events/BP_Finger_Right.Right Finger Up` (`self.RightFinger`))
      (`KismetSystemLibrary.Delay` 0.2)
      (`/Game/Blueprints/Events/BP_Finger_Left.Left Finger Down` (`self.LeftFinger`))
      (`/Game/Blueprints/Events/BP_Finger_Right.Right Finger Down` (`self.RightFinger`))
      (elif (`KismetMathLibrary.RandomBoolWithWeight` 0.5)
        (`/Game/Blueprints/Events/BP_Finger_Left.Left Finger Up` (`self.LeftFinger`))
        (`KismetSystemLibrary.Delay` 0.2)
        (`/Game/Blueprints/Events/BP_Finger_Left.Left Finger Down` (`self.LeftFinger`))
        (else
          (`/Game/Blueprints/Events/BP_Finger_Right.Right Finger Up` (`self.RightFinger`))
          (`KismetSystemLibrary.Delay` 0.2)
          (`/Game/Blueprints/Events/BP_Finger_Right.Right Finger Down` (`self.RightFinger`)))))))

(fn `UserConstructionScript`
  (`BoxComponent.SetBoxExtent` (`self.Box`) (`self.TriggerExtent`) true))