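; Cannonball projectile actor that explodes on hitting the ninja character and has the level's cannon fire again.
; BeginPlay caches the first BP_Cannon found in the level.
; A hit on BP_CH_Ninja spawns an explosion, hides the ball, fires a radial force impulse, calls FireCannon, then destroys the actor.
; Overlapping a BP_Trigger also calls FireCannon and destroys the ball, without the explosion or impulse.
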(event `self.ReceiveBeginPlay`
  (bind _outactors (`GameplayStatics.GetAllActorsOfClass` "/Game/Blueprints/Events/BP_Cannon.BP_Cannon_C"))
  (set `self.Cannon` (`|GetArrayItem` _outactors)))

(event `self.ReceiveHit`
  (params (MyComp :type "PrimitiveComponent Object Reference") (Other :type "Actor Object Reference") (OtherComp :type "PrimitiveComponent Object Reference") (bSelfMoved :type Boolean) (HitLocation :type "Vector Structure") (HitNormal :type "Vector Structure") (NormalImpulse :type "Vector Structure") (Hit :type "HitResult Structure (by ref)"))
  (cast `/Game/Blueprints/Characters/BP_CH_Ninja` Other)
  (`GameplayStatics.SpawnEmitterAtLocation` "/Game/Particles/Particles/P_Explosion_01.P_Explosion_01" (`self.K2_GetActorLocation`))
  (`SceneComponent.SetVisibility` (`self.SM_CannonBall`) false false)
  (`ActorComponent.Activate` (`self.RadialForce`) false)
  (`RadialForceComponent.FireImpulse` (`self.RadialForce`))
  (`/Game/Blueprints/Events/BP_Cannon.FireCannon` (`self.Cannon`))
  (`self.K2_DestroyActor`))

(event `self.ReceiveActorBeginOverlap`
  (params (OtherActor :type "Actor Object Reference"))
  (cast `/Game/Blueprints/BP_Trigger` OtherActor)
  (`/Game/Blueprints/Events/BP_Cannon.FireCannon` (`self.Cannon`))
  (`self.K2_DestroyActor`))

(fn `UserConstructionScript`)