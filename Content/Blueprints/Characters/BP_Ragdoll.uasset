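; BP_Ragdoll is a physics-simulated ragdoll character body tinted with one of four colors.
; On BeginPlay it enables physics simulation on its skeletal mesh and picks UsedColor from Color1 through Color4 based on ID.
; SetVectorParameter then creates a dynamic material instance for each mesh material slot and writes that color to the Color_R parameter.
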(event `self.ReceiveBeginPlay`
  (`PrimitiveComponent.SetSimulatePhysics` (`self.SkeletalMesh`) true)
  (switch `int` (`self.ID`)
    (:`0`
      (set `self.Used Color` (`self.Color1`)))
    (:`1`
      (set `self.Used Color` (`self.Color2`)))
    (:`2`
      (set `self.Used Color` (`self.Color3`)))
    (:`3`
      (set `self.Used Color` (`self.Color4`))))
  (`self.SetVectorParameter`))

(fn `SetVectorParameter`
  (for (_ _array_index) (`MeshComponent.GetMaterials` (`self.SkeletalMesh`))
    (bind _returnvalue (`PrimitiveComponent.CreateDynamicMaterialInstance` (`self.SkeletalMesh`) _array_index null))
    (`MaterialInstanceDynamic.SetVectorParameterValue` _returnvalue "Color_R" (`self.Used Color`))))

(fn `UserConstructionScript`)