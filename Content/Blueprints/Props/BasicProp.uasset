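; BasicProp is a prop actor with overlap logic meant to register it with a BP_CH_Ninja player while not picked up.
; Begin overlap filters by class, but sets LastTouchedActor to None before writing itself to that reference's StoredProp, so no ninja receives it.
; End overlap clears the leaving ninja's StoredProp and resets LastTouchedActor.
; PropAction is an empty function, and the construction script does nothing.
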(event `self.ReceiveActorBeginOverlap`
  (params (OtherActor :type "Actor Object Reference"))
  ;[1 1 1] Erstelle eine Referent zum letzten berührten Player
  (if (== OtherActor (`self.LastTouchedActor`))
    _
    (elif (not (`self.IsPickedUp`))
      (if (== (`GameplayStatics.GetObjectClass` OtherActor) null)
        (cast `/Game/Blueprints/Characters/BP_CH_Ninja` OtherActor)
        (bind _output_get (set `self.LastTouchedActor` null))
        (set `/Game/Blueprints/Characters/BP_CH_Ninja.StoredProp` self _output_get)))))

(event `self.ReceiveActorEndOverlap`
  (params (OtherActor :type "Actor Object Reference"))
  ;[1 1 1] Erstelle eine Referent zum letzten berührten Player
  (if (not (`self.IsPickedUp`))
    (bind _asbp_ch_ninja (cast `/Game/Blueprints/Characters/BP_CH_Ninja` OtherActor))
    (bind _output_get (set `self.LastTouchedActor` _asbp_ch_ninja))
    (set `/Game/Blueprints/Characters/BP_CH_Ninja.StoredProp` null _output_get)
    (set `self.LastTouchedActor` null)))

(fn `PropAction`)

(fn `UserConstructionScript`)