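; ClothBomb is a throwable prop that, while picked up, either previews its arc or launches on PropAction.
; Throwing detaches it, enables physics and applies an acceleration force along the owner mesh's right vector.
; Aiming samples a hand-written gravity equation over time steps and draws the path with one-frame debug line traces.
; TraceThrow, an alternative using projectile prediction and NavMesh projection, is only called from a second attempt that never runs.
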(event `self.PropAction`
  (params (Throw :type Boolean))
  ;[1 1 1] First Try
  (if (`self.IsPickedUp`)
    (if Throw
      (`self.K2_DetachFromActor` self "KeepWorld" "KeepWorld" "KeepWorld")
      (`PrimitiveComponent.SetSimulatePhysics` (`self.PropMesh`) true)
      (`PrimitiveComponent.AddForce` (`self.PropMesh`) (* (`SceneComponent.GetRightVector` (`Character.Mesh` (`self.PropOwner`))) (`self.ActionVelocity`)) "None" true)
      (else
        (`self.Draw Projectile Path`)
        (set `self.NewStartingVector` (`SceneComponent.K2_GetComponentLocation` (`self.PropMesh`)))))))

(fn `Draw Projectile Path`
  (bind _segmentvectors (`self.SegmentVectors`))
  (for _index (range (+ (+ (`KismetMathLibrary.FFloor` (/ (`self.PathLifeTime`) (`self.TimeInterval`))) 1) 1))
    (bind _point1 (`self.GetSegmentAtTime` (`SceneComponent.K2_GetComponentLocation` (`self.PropMesh`)) (* (`SceneComponent.GetRightVector` (`Character.Mesh` (`self.PropOwner`))) (`self.ActionVelocity`)) (0.0 0.0 -450000.0) (* _index (`self.TimeInterval`)) (* (+ _index 1) (`self.TimeInterval`))))
    (`KismetArrayLibrary.Array_Add` (`self.SegmentVectors`) _point1))
  (for _index_2 (range (`KismetArrayLibrary.Array_Length` (`self.SegmentVectors`)))
    (`KismetSystemLibrary.LineTraceSingle` :`Start` (`|GetArrayItem` _segmentvectors _index_2) :`End` (`|GetArrayItem` _segmentvectors (+ _index_2 1)) :`TraceChannel` "TraceTypeQuery1" :`DrawDebugType` "ForOneFrame" :`bIgnoreSelf` false :`DrawTime` (`self.PathLifeTime`)))
  (`KismetArrayLibrary.Array_Clear` (`self.SegmentVectors`)))

(fn `GetSegmentAtTime`
  (params (StartLocation :type "Vector Structure") (InitialVelocity :type "Vector Structure") (Gravity :type "Vector Structure") (Time1 :type "Float (double-precision)") (Time2 :type "Float (double-precision)"))
  (returns (Point1 :type "Vector Structure") (Point2 :type "Vector Structure"))
  (return (+ StartLocation (* InitialVelocity Time1) (* Gravity (* Time1 Time1 0.5))) (+ StartLocation (* InitialVelocity 0.0) (* Gravity (* Time2 Time2 0.5)))))

(fn `TraceThrow`
  (returns (TracePoints :type "Array of Vector Structure") (NavMeshLocation :type "Vector Structure") (TraceLocation :type "Vector Structure") (Success :type Boolean))
  (locals (`Project Nav Extends` :type "Float (double-precision)" :default 500.0))
  (bind _project_nav_extends (`local.Project Nav Extends`))
  (bind _rootcomponent (`Actor.RootComponent` (`self.PropOwner`)))
  (bind (_outhit _outpathpositions _outlasttracedestination _returnvalue) (`GameplayStatics.Blueprint_PredictProjectilePath_ByObjectType` :`StartPos` (`SceneComponent.K2_GetComponentLocation` _rootcomponent) :`LaunchVelocity` (* (`SceneComponent.GetForwardVector` _rootcomponent) (`self.ActionVelocity`)) :`ObjectTypes` (`|MakeArray` "ObjectTypeQuery1" :!type "EObjectTypeQuery Enum") :`SimFrequency` 30.0)) ; Simuliere das werfen des Projektils (mit gravitation) um den Treefferpunkt zu finden
  (bind (_bblockinghit _binitialoverlap _time _distance _location) (`GameplayStatics.BreakHitResult` _outhit))
  (bind (_projectedlocation _returnvalue_2) (`NavigationSystem.K2_ProjectPointToNavigation` (`NavigationSystem.GetNavigationSystem`) _location null null (`KismetMathLibrary.MakeVector` _project_nav_extends _project_nav_extends _project_nav_extends)))
  (return _outpathpositions _projectedlocation _location (and _returnvalue _returnvalue_2)))

(fn `UserConstructionScript`
  (`parent.UserConstructionScript`))