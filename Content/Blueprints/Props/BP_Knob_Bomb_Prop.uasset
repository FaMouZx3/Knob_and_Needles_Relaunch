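; Knob bomb prop that a ninja character can pick up, carry in the right hand and throw as a timed explosive.
; BombEvent toggles between snapping the mesh to the hand socket and throwing it via ProjectileMovement along the character mesh's right vector with an upward arc.
; The impulse radius collides only after the throw.
; After a short fuse, it explodes with particles and a radial impulse, damages overlapping ninjas and destroys itself.
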(event `self.ReceiveBeginPlay`
  ;[1 1 1] Deaktivieren von Collision damit Character nicht an der Kollision hängen bleibt
  (`PrimitiveComponent.SetCollisionEnabled` (`self.ImpulsRadius`) "NoCollision"))

(event `BombEvent`
  (params (NinjaRef :type "/Game/Blueprints/Characters/BP_CH_Ninja Object Reference"))
  ;[1 1 1] Attach Bombe to Character
  (if (not (`self.IsSnapped`))
    (bind _output_get (set `self.CharacterRef` NinjaRef))
    (set `/Game/Blueprints/Characters/BP_CH_Ninja.IsThrow` true _output_get)
    (set `self.IsSnapped` true)
    (`PrimitiveComponent.SetSimulatePhysics` (`self.BombMesh`) false)
    (`SceneComponent.K2_AttachToComponent` (`self.BombMesh`) (`/Game/Blueprints/Characters/BP_CH_Ninja.RightHandHitbox` (`self.CharacterRef`)) "Right_Hand_Prop_Grab" "SnapToTarget" "SnapToTarget" "KeepWorld" false)
    (else
      (`self.BombThrow`))))

(event `BombThrow`
  (bind (_returnvalue_x _returnvalue_y _returnvalue_z) (`KismetMathLibrary.BreakVector` (`SceneComponent.GetRightVector` (`Character.Mesh` (`self.CharacterRef`)))))
  ;[1 1 1] Throw Bomb Event
  (set `/Game/Blueprints/Characters/BP_CH_Ninja.IsThrow` false (`self.CharacterRef`))
  (`self.K2_DetachFromActor` "KeepWorld" "KeepWorld" "KeepWorld")
  (set `MovementComponent.Velocity` (`KismetMathLibrary.MakeVector` (* _returnvalue_x 1000.0) (* _returnvalue_y 1000.0) (* (+ _returnvalue_z 1.0) 1000.0)) (`self.ProjectileMovement`))
  (`ActorComponent.Activate` (`self.ProjectileMovement`) false)
  (`PrimitiveComponent.SetCollisionEnabled` (`self.ImpulsRadius`) "QueryOnly")
  (`KismetSystemLibrary.Delay` 2.0)
  (`GameplayStatics.SpawnEmitterAtLocation` "/Game/Particles/Particles/P_Explosion_01.P_Explosion_01" (`self.K2_GetActorLocation`) (struct) (3.0 3.0 3.0))
  (`SceneComponent.SetVisibility` (`self.BombMesh`) false false)
  (`ActorComponent.Activate` (`self.RadialForce`) false)
  (`RadialForceComponent.FireImpulse` (`self.RadialForce`))
  (for _array_element (`PrimitiveComponent.GetOverlappingActors` (`self.ImpulsRadius`) "/Game/Blueprints/Characters/BP_CH_Ninja.BP_CH_Ninja_C")
    (bind _asbp_ch_ninja (cast `/Game/Blueprints/Characters/BP_CH_Ninja` _array_element))
    (set `/Game/Blueprints/Characters/BP_CH_Ninja.Health` (- (`/Game/Blueprints/Characters/BP_CH_Ninja.Health` _asbp_ch_ninja) 5) _asbp_ch_ninja))
  (`self.K2_DestroyActor`))

(fn `UserConstructionScript`)