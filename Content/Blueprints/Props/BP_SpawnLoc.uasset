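; BP_SpawnLoc is a placeable spawner that keeps knob bomb props dropping into a defined area.
; BeginPlay reads two marker cubes as the area's min and max corners and starts a looping one-second timer.
; Each tick counts all BP_Knob_Bomb_Prop actors in the world and, unless exactly three exist, spawns another at a random XY between the markers, raised by SpawnHeight above the spawner.
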(event `self.ReceiveBeginPlay`
  (set `self.MinLoc` (`SceneComponent.K2_GetComponentLocation` (`self.MinLocCube`)))
  (set `self.MaxLoc` (`SceneComponent.K2_GetComponentLocation` (`self.MaxLocCube`)))
  (`KismetSystemLibrary.K2_SetTimer` null "SpawnBomb" 1.0 true))

(fn `SpawnBomb`
  (bind (_returnvalue_x _returnvalue_y _returnvalue_z) (`KismetMathLibrary.BreakVector` (`self.K2_GetActorLocation`)))
  (bind (_minloc_x _minloc_y) (`KismetMathLibrary.BreakVector` (`self.MinLoc`)))
  (bind (_maxloc_x _maxloc_y) (`KismetMathLibrary.BreakVector` (`self.MaxLoc`)))
  (bind _outactors (`GameplayStatics.GetAllActorsOfClass` "/Game/Blueprints/Props/BP_Knob_Bomb_Prop.BP_Knob_Bomb_Prop_C"))
  (if (not (== (`KismetArrayLibrary.Array_Length` _outactors) 3))
    (`|SpawnActorFromClass` "/Game/Blueprints/Props/BP_Knob_Bomb_Prop.BP_Knob_Bomb_Prop_C" (`KismetMathLibrary.MakeTransform` (`KismetMathLibrary.MakeVector` (`KismetMathLibrary.RandomFloatInRange` _minloc_x _maxloc_x) (`KismetMathLibrary.RandomFloatInRange` _minloc_y _maxloc_y) (+ _returnvalue_z (`self.SpawnHeight`)))) "Undefined" "OverrideRootScale" null null)))

(fn `UserConstructionScript`)