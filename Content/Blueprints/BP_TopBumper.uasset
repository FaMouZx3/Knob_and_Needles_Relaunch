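; BP_TopBumper is a pinball bumper that knocks the ball away and flashes when hit.
; On BeginPlay it creates a dynamic instance of M_Bumper on its static mesh.
; When a Pinball overlaps its sphere, it applies a strong impulse to the ball, directed away from the bumper's center.
; It also raises the material's EStrength parameter, then restores it after a one-second delay.
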(event `self.ReceiveBeginPlay`
  (bind _returnvalue (`PrimitiveComponent.CreateDynamicMaterialInstance` (`self.StaticMesh`) 0 "/Game/Meshes/Environment/Pinball/M_Bumper.M_Bumper"))
  (set `self.BumperDynaMat` _returnvalue))

(event `self.Sphere.OnComponentBeginOverlap`
  (params (OverlappedComponent :type "PrimitiveComponent Object Reference") (OtherActor :type "Actor Object Reference") (OtherComp :type "PrimitiveComponent Object Reference") (OtherBodyIndex :type Integer) (bFromSweep :type Boolean) (SweepResult :type "HitResult Structure (by ref)"))
  (bind _aspinball (cast `/Game/Blueprints/Pinball` OtherActor))
  (`PrimitiveComponent.AddImpulse` (`/Game/Blueprints/Pinball.Sphere` _aspinball) (* (`KismetMathLibrary.Normal` (- (`self.K2_GetActorLocation` OtherActor) (`self.K2_GetActorLocation`))) 300000.0) "None" false)
  (`MaterialInstanceDynamic.SetScalarParameterValue` (`self.BumperDynaMat`) "EStrength" 20.0)
  (`KismetSystemLibrary.Delay` 1.0)
  (`MaterialInstanceDynamic.SetScalarParameterValue` (`self.BumperDynaMat`) "EStrength" 1.0))

(fn `UserConstructionScript`)