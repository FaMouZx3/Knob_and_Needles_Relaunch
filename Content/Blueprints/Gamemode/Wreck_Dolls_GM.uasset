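; Game mode for local multiplayer Wreck Dolls that spawns players and handles pausing.
; BeginPlay removes the default player, then creates KnAInstance's PlayerCount players, each with its own health widget.
; Each ninja gets a PlayerID, saved customizations through per-player macros, and its player color.
; Pausing swaps all widgets for UI_Pause; unpausing removes it and recreates health widgets without adding them to the viewport.
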(event `self.ReceiveBeginPlay`
  (`GameplayStatics.RemovePlayer` (`GameplayStatics.GetPlayerController` 0) true)
  (set `self.WidgetArray` (`|MakeArray` "/Game/Blueprints/Widgets/IngameWidgets/UI_Health_PlayerOne.UI_Health_PlayerOne_C" "/Game/Blueprints/Widgets/IngameWidgets/UI_Health_PlayerTwo.UI_Health_PlayerTwo_C" "/Game/Blueprints/Widgets/IngameWidgets/UI_Health_playerThree.UI_Health_playerThree_C" "/Game/Blueprints/Widgets/IngameWidgets/UI_Health_PlayerFour.UI_Health_PlayerFour_C" :!type "UserWidget Class Reference"))
  (bind _askn_ainstance (cast `/Game/Blueprints/Gamemode/KnAInstance` (`GameplayStatics.GetGameInstance`)))
  (for _index (range (`/Game/Blueprints/Gamemode/KnAInstance.PlayerCount` _askn_ainstance))
    (bind _returnvalue (`GameplayStatics.CreatePlayer` _index))
    (bind _returnvalue_2 (`|CreateWidget` (`|GetArrayItem` (`self.WidgetArray`) _index) _returnvalue))
    (`UserWidget.AddToViewport` _returnvalue_2 0)
    (bind _asbp_ch_ninja (cast `/Game/Blueprints/Characters/BP_CH_Ninja` (`GameplayStatics.GetPlayerCharacter` _index)))
    (set `self.NinjaRef` _asbp_ch_ninja)
    (bind _output_get (set `/Game/Blueprints/Characters/BP_CH_Ninja.PlayerID` _index _asbp_ch_ninja))
    (switch `int` _output_get
      (:`0`
        (bind _askn_ainstance_2 (cast `/Game/Blueprints/Gamemode/KnAInstance` (`GameplayStatics.GetGameInstance`)))
        (`/Game/Blueprints/Characters/BP_CH_Ninja.SetCustomizables` (`self.NinjaRef`) (`/Game/Blueprints/Gamemode/KnAInstance.Player1Customs` _askn_ainstance_2)))
      (:`1`
        (bind _askn_ainstance_3 (cast `/Game/Blueprints/Gamemode/KnAInstance` (`GameplayStatics.GetGameInstance`)))
        (`/Game/Blueprints/Characters/BP_CH_Ninja.SetCustomizables` (`self.NinjaRef`) (`/Game/Blueprints/Gamemode/KnAInstance.Player2Customs` _askn_ainstance_3)))
      (:`2`
        (bind _askn_ainstance_4 (cast `/Game/Blueprints/Gamemode/KnAInstance` (`GameplayStatics.GetGameInstance`)))
        (`/Game/Blueprints/Characters/BP_CH_Ninja.SetCustomizables` (`self.NinjaRef`) (`/Game/Blueprints/Gamemode/KnAInstance.Player3Customs` _askn_ainstance_4)))
      (:`3`
        (bind _askn_ainstance_5 (cast `/Game/Blueprints/Gamemode/KnAInstance` (`GameplayStatics.GetGameInstance`)))
        (`/Game/Blueprints/Characters/BP_CH_Ninja.SetCustomizables` (`self.NinjaRef`) (`/Game/Blueprints/Gamemode/KnAInstance.Player4Customs` _askn_ainstance_5))))
    (`/Game/Blueprints/Characters/BP_CH_Ninja.SetPlayerColor` (`self.NinjaRef`))))

(fn `PauseGame`
  (returns (PauseWidgetref :type "/Game/Blueprints/Widgets/MenuWidgets/UI_Pause Object Reference"))
  (`GameplayStatics.SetGamePaused` true)
  (`WidgetLayoutLibrary.RemoveAllWidgets`)
  (bind _returnvalue (`|CreateWidget` "/Game/Blueprints/Widgets/MenuWidgets/UI_Pause.UI_Pause_C" (`GameplayStatics.GetPlayerController` 0)))
  (set `self.Active Widget` _returnvalue)
  (`UserWidget.AddToViewport` _returnvalue 0)
  (return _returnvalue))

(fn `UnPauseGame`
  (`GameplayStatics.SetGamePaused` false)
  (`WidgetLayoutLibrary.RemoveAllWidgets`)
  (bind _askn_ainstance (cast `/Game/Blueprints/Gamemode/KnAInstance` (`GameplayStatics.GetGameInstance`)))
  (for _index (range (`/Game/Blueprints/Gamemode/KnAInstance.PlayerCount` _askn_ainstance))
    (`|CreateWidget` (`|GetArrayItem` (`self.WidgetArray`) _index))))

(fn `UserConstructionScript`)