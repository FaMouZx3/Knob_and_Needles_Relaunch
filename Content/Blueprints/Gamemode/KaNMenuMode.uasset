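; Menu game mode that switches between main, character selection, credits and controls screens, and opens the pinball map behind a loading screen.
; On BeginPlay it shows the main menu and points the first player's view at the first camera found.
; Each load function clears all widgets, and menu screens record the active widget and enum.
; Character selection also creates four local players, moving their pawns to index-tagged actors and setting their colors.
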(event `self.ReceiveBeginPlay`
  (`self.loadMain`)
  (bind _outactors (`GameplayStatics.GetAllActorsOfClass` "/Game/Blueprints/Menu/camera.camera_C"))
  (`PlayerController.SetViewTargetWithBlend` (`GameplayStatics.GetPlayerController` 0) (`|GetArrayItem` _outactors) 0.0 "VTBlend_Linear" 0.0 false))

(fn `loadCharselection`
  (`WidgetLayoutLibrary.RemoveAllWidgets`)
  (bind _returnvalue (`|CreateWidget` "/Game/Blueprints/Widgets/MenuWidgets/UI_CharSelectionWidget.UI_CharSelectionWidget_C" (`GameplayStatics.GetPlayerController` 0)))
  (`UserWidget.AddToViewport` _returnvalue 0)
  (set `self.activeWidget` _returnvalue)
  (set `self.activWidgetEnum` "NewEnumerator1")
  (for _index (range 4)
    (`GameplayStatics.CreatePlayer` _index))
  (`self.SetPlayerPosition`))

(fn `loadControls`
  (`WidgetLayoutLibrary.RemoveAllWidgets`)
  (bind _returnvalue (`|CreateWidget` "/Game/Blueprints/Widgets/MenuWidgets/UI_ControlsWidget.UI_ControlsWidget_C" (`GameplayStatics.GetPlayerController` 0)))
  (`UserWidget.AddToViewport` _returnvalue 0)
  (set `self.activeWidget` _returnvalue)
  (set `self.activWidgetEnum` "NewEnumerator3"))

(fn `loadCredits`
  (`WidgetLayoutLibrary.RemoveAllWidgets`)
  (bind _returnvalue (`|CreateWidget` "/Game/Blueprints/Widgets/MenuWidgets/UI_CreditWidget.UI_CreditWidget_C" (`GameplayStatics.GetPlayerController` 0)))
  (`UserWidget.AddToViewport` _returnvalue 0)
  (set `self.activeWidget` _returnvalue)
  (set `self.activWidgetEnum` "NewEnumerator2"))

(fn `LoadGame`
  (`WidgetLayoutLibrary.RemoveAllWidgets`)
  (bind _returnvalue (`|CreateWidget` "/Game/Blueprints/Widgets/MenuWidgets/UI_LoadingScreenWidget.UI_LoadingScreenWidget_C" (`GameplayStatics.GetPlayerController` 0)))
  (`UserWidget.AddToPlayerScreen` _returnvalue 0)
  (`GameplayStatics.OpenLevel` "map_Pinball"))

(fn `loadMain`
  (`WidgetLayoutLibrary.RemoveAllWidgets`)
  (bind _returnvalue (`|CreateWidget` "/Game/Blueprints/Widgets/MenuWidgets/UI_MainWidget.UI_MainWidget_C" (`GameplayStatics.GetPlayerController` 0)))
  (`UserWidget.AddToViewport` _returnvalue 0)
  (set `self.activeWidget` _returnvalue)
  (set `self.activWidgetEnum` "NewEnumerator0"))

(fn `SetPlayerPosition`
  (bind _outactors (`GameplayStatics.GetAllActorsOfClass` "/Game/Blueprints/Menu/tempmenuplayer.tempmenuplayer_C"))
  (for (_array_element _array_index) _outactors
    (set `/Game/Blueprints/Menu/tempmenuplayer.playercontrollerID` _array_index _array_element)
    (bind _outactors_2 (`GameplayStatics.GetAllActorsWithTag` (`KismetStringLibrary.Conv_StringToName` (`KismetStringLibrary.BuildString_Int` "" "" _array_index))))
    (bind _returnvalue_location (`KismetMathLibrary.BreakTransform` (`self.GetTransform` (`|GetArrayItem` _outactors_2))))
    (`self.K2_SetActorLocation` _array_element _returnvalue_location false false)
    (`/Game/Blueprints/Menu/tempmenuplayer.SetPlayerColor` _array_element)))

(fn `UserConstructionScript`)