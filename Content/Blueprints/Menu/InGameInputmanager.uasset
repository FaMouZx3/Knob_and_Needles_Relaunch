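; In-game input manager for Wreck Dolls that drives the pause menu and end-of-match screen from player input.
; CastInput routes each input by state: Start pauses via the game mode, and only the pausing player can navigate, resume or quit.
; Selection changes play the pause widget's ResumeToQuit animation forward or reversed.
; PlayerWon passes the winner to the game mode's win screen, where any player's Fire or Back loads the main menu.
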(fn `cast Input`
  (params (`player ID` :type Integer) (Input :type "/Game/Blueprints/Menu/Inputs Enum" :default "NewEnumerator0"))
  (locals (tmpinput :type "/Game/Blueprints/Menu/Inputs Enum") (tmpPlayerID :type Integer))
  (set `local.tmpPlayerID` `player ID`)
  (set `local.tmpinput` Input)
  (if (`self.Gamepaused`)
    (if (`self.GameEnd`)
      (switch `/Game/Blueprints/Menu/Inputs` (`local.tmpinput`)
        (:`NewEnumerator0`
          _)
        (:`NewEnumerator1`
          _))
      (bind _aswreck_dolls_gm (cast `/Game/Blueprints/Gamemode/Wreck_Dolls_GM` (`GameplayStatics.GetGameMode`)))
      (`/Game/Blueprints/Gamemode/Wreck_Dolls_GM.LoadMainMenu` _aswreck_dolls_gm)
      (elif (== (`local.tmpPlayerID`) (`self.activeplayer`))
        (switch `/Game/Blueprints/Menu/Inputs` (`local.tmpinput`)
          (:`NewEnumerator0`
            (switch `int` (`self.activeSelection`)
              (:`0`
                (`self.UnPauseGame`))
              (:`1`
                (bind _aswreck_dolls_gm_2 (cast `/Game/Blueprints/Gamemode/Wreck_Dolls_GM` (`GameplayStatics.GetGameMode`)))
                (`/Game/Blueprints/Gamemode/Wreck_Dolls_GM.LoadMainMenu` _aswreck_dolls_gm_2))))
          (:`NewEnumerator1`
            (`self.UnPauseGame` :!label _label))
          (:`NewEnumerator3`
            (if (!= (`self.activeSelection`) 0)
              (set `self.activeSelection` 0)
              (`UserWidget.PlayAnimation` (`self.PausWidgetRef`) (`/Game/Blueprints/Widgets/MenuWidgets/UI_Pause.ResumeToQuit` (`self.PausWidgetRef`)) 0.0 1 "Reverse" 2.0)))
          (:`NewEnumerator4`
            (if (!= (`self.activeSelection`) 1)
              (set `self.activeSelection` 1)
              (`UserWidget.PlayAnimation` (`self.PausWidgetRef`) (`/Game/Blueprints/Widgets/MenuWidgets/UI_Pause.ResumeToQuit` (`self.PausWidgetRef`)) 0.0 1 "Forward" 2.0)))
          (:`NewEnumerator7`
            (goto _label)))))
    (else
      (switch `/Game/Blueprints/Menu/Inputs` (`local.tmpinput`)
        (:`NewEnumerator7`
          (set `self.Gamepaused` true)
          (set `self.activeplayer` (`local.tmpPlayerID`))
          (bind _aswreck_dolls_gm_3 (cast `/Game/Blueprints/Gamemode/Wreck_Dolls_GM` (`GameplayStatics.GetGameMode`)))
          (bind _pausewidgetref (`/Game/Blueprints/Gamemode/Wreck_Dolls_GM.PauseGame` _aswreck_dolls_gm_3))
          (set `self.PausWidgetRef` _pausewidgetref))))))

(fn `PlayerWon`
  (params (PlayerWon :type Integer))
  (set `self.Gamepaused` true)
  (set `self.GameEnd` true)
  (bind _aswreck_dolls_gm (cast `/Game/Blueprints/Gamemode/Wreck_Dolls_GM` (`GameplayStatics.GetGameMode`)))
  (set `/Game/Blueprints/Gamemode/Wreck_Dolls_GM.WinnerID` PlayerWon _aswreck_dolls_gm)
  (`/Game/Blueprints/Gamemode/Wreck_Dolls_GM.WinScreen` _aswreck_dolls_gm))

(fn `UnPauseGame`
  (set `self.Gamepaused` false)
  (bind _aswreck_dolls_gm (cast `/Game/Blueprints/Gamemode/Wreck_Dolls_GM` (`GameplayStatics.GetGameMode`)))
  (`/Game/Blueprints/Gamemode/Wreck_Dolls_GM.UnPauseGame` _aswreck_dolls_gm))

(fn `UserConstructionScript`)