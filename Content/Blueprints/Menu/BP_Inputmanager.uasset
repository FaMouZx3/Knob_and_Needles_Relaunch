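; BP_Inputmanager is a menu input router that passes a player's ID and input to the currently active menu screen.
; CastInput reads the active widget enum from KaNMenuMode, casts the active widget to the matching class and calls its GetInput.
; Main menu, character selection and map selection receive input, with only character selection's GetInput result captured for the return value.
; Settings and credits only perform the cast and forward nothing.
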(fn `cast Input`
  (params (player :type Integer) (Inputs :type "/Game/Blueprints/Menu/EN_Inputs Enum" :default "NewEnumerator0"))
  (returns (NewParam :type "/Game/Blueprints/Menu/ST_CharCustomizables Structure"))
  (locals (playerID :type Integer) (Input :type "/Game/Blueprints/Menu/EN_Inputs Enum") (playerref1 :type "/Game/Blueprints/Menu/tempmenuplayer Object Reference"))
  (bind _input (`local.Input`))
  (bind _playerid (`local.playerID`))
  (set `local.playerID` player)
  (set `local.Input` Inputs)
  (bind _aska_nmenu_mode (cast `/Game/Blueprints/Gamemode/KaNMenuMode` (`GameplayStatics.GetGameMode`)))
  (switch `/Game/Blueprints/Menu/EN_MenüState` (`/Game/Blueprints/Gamemode/KaNMenuMode.activWidgetEnum` _aska_nmenu_mode)
    (:`NewEnumerator0`
      (bind _activewidget (`/Game/Blueprints/Gamemode/KaNMenuMode.activeWidget` _aska_nmenu_mode))
      (bind _asui_main_widget (cast `/Game/Blueprints/Widgets/MenuWidgets/UI_MainWidget` _activewidget))
      (`/Game/Blueprints/Widgets/MenuWidgets/UI_MainWidget.GetInput` _asui_main_widget _playerid _input)
      (return (stale _playerstruct)))
    (:`NewEnumerator1`
      (bind _asui_char_selection_widget (cast `/Game/Blueprints/Widgets/MenuWidgets/UI_CharSelectionWidget` _activewidget))
      (bind _playerstruct (`/Game/Blueprints/Widgets/MenuWidgets/UI_CharSelectionWidget.GetInput` _asui_char_selection_widget _playerid _input))
      (return _playerstruct))
    (:`NewEnumerator4`
      (bind _asui_map_selection_widget (cast `/Game/Blueprints/Widgets/MenuWidgets/UI_MapSelectionWidget` _activewidget))
      (`/Game/Blueprints/Widgets/MenuWidgets/UI_MapSelectionWidget.GetInput` _asui_map_selection_widget _playerid _input)
      (return _playerstruct))
    (:`NewEnumerator3`
      (cast `/Game/Blueprints/Widgets/MenuWidgets/UI_SettingWidget` _activewidget))
    (:`NewEnumerator2`
      (cast `/Game/Blueprints/Widgets/MenuWidgets/UI_CreditWidget` _activewidget))))

(fn `UserConstructionScript`)