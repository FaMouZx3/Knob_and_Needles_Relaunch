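; Temporary menu player that relays a player's directional, Fire, start and Back presses to the Inputmanager.
; On BeginPlay it caches the first Inputmanager, resets its player ID to 0 and snaps to the actor tagged with that controller's ID.
; Each press sets an input enum and funnels into one shared CastInput call that passes the player ID and input.
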(event `self.ReceiveBeginPlay`
  (bind _outactors (`GameplayStatics.GetAllActorsOfClass` "/Game/Blueprints/Menu/inputmanager.inputmanager_C"))
  (set `self.inputController` (`|GetArrayItem` _outactors))
  (`KismetSystemLibrary.PrintString` (`KismetStringLibrary.Conv_IntToString` (`self.playercontrollerID`)))
  (bind _output_get (set `self.playercontrollerID` 0))
  (bind _returnvalue (`GameplayStatics.GetPlayerControllerID` (`GameplayStatics.GetPlayerController` _output_get)))
  (bind _outactors_2 (`GameplayStatics.GetAllActorsWithTag` (`KismetStringLibrary.Conv_StringToName` (`KismetStringLibrary.BuildString_Int` "" "" _returnvalue))))
  (`self.K2_SetActorTransform` (`self.GetTransform` (`|GetArrayItem` _outactors_2))))

(event `Key|Up`
  (params (Key :type "Key Structure"))
  (:`Pressed`
    (set `self.pressedInput` "NewEnumerator3")
    (`/Game/Blueprints/Menu/inputmanager.castInput` (`self.inputController`) (`self.playercontrollerID`) (`self.pressedInput`) :!label _label)))

(event `Key|Down`
  (params (Key :type "Key Structure"))
  (:`Pressed`
    (set `self.pressedInput` "NewEnumerator4")
    (goto _label)))

(event `InputAction|Fire`
  (params (Key :type "Key Structure"))
  (:`Pressed`
    (set `self.pressedInput` "NewEnumerator0")
    (goto _label)))

(event `Key|Left`
  (params (Key :type "Key Structure"))
  (:`Pressed`
    (set `self.pressedInput` "NewEnumerator5")
    (goto _label)))

(event `Key|Right`
  (params (Key :type "Key Structure"))
  (:`Pressed`
    (set `self.pressedInput` "NewEnumerator6")
    (goto _label)))

(event `InputAction|start`
  (params (Key :type "Key Structure"))
  (:`Pressed`
    (set `self.pressedInput` "NewEnumerator7")
    (goto _label)))

(event `InputAction|Back`
  (params (Key :type "Key Structure"))
  (:`Pressed`
    (set `self.pressedInput` "NewEnumerator1")
    (goto _label)))

(fn `UserConstructionScript`)