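; BP_Helper is a menu helper with a single function, ChangeIndex, that steps an index by one within zero to MaxIndex.
; The Circle flag chooses between wrapping to the opposite end and clamping at the limit.
; The IncreasIndex flag works opposite to its name: true decrements the index and false increments it.
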(fn `ChangeIndex`
  (params (IncreasIndex :type Boolean) (index :type Integer) (MaxIndex :type Integer) (Circle :type Boolean))
  (returns (outIndex :type Integer))
  (locals (tmpIndex :type Integer) (CustomHeadArray :type "Array of StaticMesh Object Reference") (CustomFaceArray :type "Array of StaticMesh Object Reference") (CustomNeckArray :type "Array of StaticMesh Object Reference") (CustomLeftArmArray :type "Array of StaticMesh Object Reference") (CustomRightArmArray :type "Array of StaticMesh Object Reference") (CustomLeftKneeArray :type "Array of StaticMesh Object Reference") (CustomRightKneeArray :type "Array of StaticMesh Object Reference") (CustomLeftFeetArray :type "Array of StaticMesh Object Reference") (CustomRightFeetArray :type "Array of StaticMesh Object Reference"))
  (if IncreasIndex
    (bind _output_get (set `local.tmpIndex` (- index 1)))
    (if (< _output_get 0)
      (if Circle
        (set `local.tmpIndex` MaxIndex)
        (else
          (set `local.tmpIndex` 0))))
    (else
      (bind _output_get_2 (set `local.tmpIndex` (+ index 1)))
      (if (> _output_get_2 MaxIndex)
        (if Circle
          (set `local.tmpIndex` 0)
          (else
            (set `local.tmpIndex` MaxIndex))))))
  (return (`local.tmpIndex`)))