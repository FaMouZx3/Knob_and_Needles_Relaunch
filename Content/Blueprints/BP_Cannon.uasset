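; BP_Cannon is a cannon actor that swings side to side and launches Pinball actors.
; On BeginPlay, the Cannon_rotation timeline drives its yaw within a fixed arc around the starting heading.
; FireCannon spawns a Pinball at the Scene component and applies an impulse along the mesh's forward vector, scaled by CanonForce.
; A timed auto-fire branch is disconnected from Tick, so nothing in this graph actively triggers firing.
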(event `self.ReceiveBeginPlay`
  (bind (_returnvalue_roll _returnvalue_pitch _returnvalue_yaw) (`KismetMathLibrary.BreakRotator` (`self.K2_GetActorRotation`)))
  (bind _yaw (`self.Yaw`))
  (set `self.Yaw` _returnvalue_yaw)
  (bind (_direction _can_rot) (`Timeline|Cannon_rotation`)
    (:`Update`
      (`self.K2_SetActorRotation` (`KismetMathLibrary.MakeRotator` 0.0 0.0 (`KismetMathLibrary.Lerp` (+ _yaw -30.0) (+ _yaw 30.0) _can_rot))))))

(event `FireCannon`
  (bind _returnvalue (`|SpawnActorFromClass` "/Game/Blueprints/Pinball.Pinball_C" (`SceneComponent.K2_GetComponentToWorld` (`self.Scene`)) "Undefined" "OverrideRootScale" null null))
  (`PrimitiveComponent.AddImpulse` (`/Game/Blueprints/Pinball.Sphere` _returnvalue) (* (`SceneComponent.GetForwardVector` (`self.StaticMesh`)) (`self.CanonForce`)) "None" false))

(event `self.ReceiveTick`
  (params (DeltaSeconds :type "Float (single-precision)")))

(fn `UserConstructionScript`)